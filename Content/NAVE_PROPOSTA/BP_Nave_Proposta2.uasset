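; Player ship pawn for a shooter: flies, fires, drops bombs and takes damage.
; BeginPlay plays a rise-and-spin timeline; Tick applies input-smoothed speeds with swept movement and banking, while hits rebound along the impact normal.
; PickupTypes selects single shot, held-fire machine gun looping on a retriggerable delay, or three-way spread; bombs consume pickups.
; Damage grants brief invincibility; zero health triggers explosion, camera shake and GameMode game over.
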(event `self.ReceiveBeginPlay`
  (bind _spawnlocation (`self.SpawnLocation`))
  ;[1 0.8776 0.08731] Spawn
  (bind _asgame_mode_bp (cast `/Game/Blueprints/GameMode_BP` (`GameplayStatics.GetGameMode`)))
  (set `self.BP_GameMode` _asgame_mode_bp)
  (set `self.Roll` (.yaw (`self.K2_GetActorRotation`)))
  (set `self.SpawnLocation` (`self.K2_GetActorLocation`))
  (bind (_direction _speed) (`Timeline|SpawnAnimation`)
    (:`Update`
      (`self.K2_SetActorLocation` (`KismetMathLibrary.VLerp` _spawnlocation (+ _spawnlocation (0.0 0.0 60.0)) _speed))
      (`self.K2_SetActorRotation` (`KismetMathLibrary.RLerp` (struct) (`KismetMathLibrary.MakeRotator` (+ (`self.Roll`) (`self.SpawnSpinCount`))) _speed)))
    (:`Finished`
      (set `self.MoveEnabled` true))))

(event `self.ReceiveTick`
  (params (DeltaSeconds :type "Float (single-precision)"))
  ;[0.1006 0 1] Movement
  (set `self.DeltaSeconds` DeltaSeconds)
  (`self.K2_SetActorLocation` (+ (`self.K2_GetActorLocation`) (`KismetMathLibrary.MakeVector` (`self.VertSpeed`) (`self.HozSpeed`))) true)
  (`self.K2_SetActorRotation` (`KismetMathLibrary.RInterpTo_Constant` (`self.K2_GetActorRotation`) (`KismetMathLibrary.MakeRotator` (+ (* (`self.HozSpeed`) 7.0) (`self.Roll`))) (`self.DeltaSeconds`) 800.0)))

(event `InputAxis|Mover_Cima_Embaixo`
  (params (AxisValue :type "Float (single-precision)"))
  ;[0.04042 1 0] Player input
  (bind _returndirectionspeed (`self.Movement` (`self.VertSpeed`) AxisValue))
  (set `self.VertSpeed` _returndirectionspeed))

(event `InputAxis|Mover`
  (params (AxisValue :type "Float (single-precision)"))
  ;[0.04042 1 0] Player input
  (bind _returndirectionspeed (`self.Movement` (`self.HozSpeed`) AxisValue))
  (set `self.HozSpeed` _returndirectionspeed))

(event `InputAction|Bomba`
  (params (Key :type "Key Structure"))
  ;[1 0.06202 0] Player Atirar - > Picks Ups tbm
  (:`Pressed`
    (if (>= (`self.PickupBomba`) 1)
      (set `self.PickupBomba` (- (`self.PickupBomba`) 1))
      (if true
        (`|SpawnActorFromClass` "/Game/Bomba/Bomba.Bomba_C" (`KismetMathLibrary.MakeTransform` (+ (`self.K2_GetActorLocation`) (`KismetMathLibrary.GreaterGreater_VectorRotator` (`self.BombaOffset`) (`self.GetControlRotation`))) (`self.K2_GetActorRotation`)) "Undefined" "OverrideRootScale" null null)
        (`self.BombExplosion` (`SceneComponent.K2_GetComponentToWorld` (`self.BombaExplosion`)))))))

(event `PrimFire`
  ;[1 0.06202 0] Player Atirar - > Picks Ups tbm
  ;;[1 1 1] Tiro  Padrao
  (`self.PrimaryFire` (`SceneComponent.K2_GetComponentToWorld` (`self.ProjectileSpawn`)) :!label _label))

(event `InputAction|PrimaryFire`
  (params (Key :type "Key Structure"))
  ;[1 0.06202 0] Player Atirar - > Picks Ups tbm
  (:`Pressed`
    (set `self.TaApertado?` true)
    (if (<= (`self.PickupTypes`) 0)
      (goto _label)
      (else
        (switch `int` (`self.PickupTypes`)
          (:`1`
            ;;[1 1 1] Metralhadora
            (`self.MachineGun` (`SceneComponent.K2_GetComponentToWorld` (`self.ProjectileSpawnMachineGun`)) :!label _label_2)
            (`KismetSystemLibrary.RetriggerableDelay` 0.1)
            (if (== (`self.PickupTypes`) 1)
              (if (`self.TaApertado?`)
                (goto _label_2))
              (else
                (set `self.TaApertado?` false))))
          (:`2`
            ;;[1 1 1] Espalhadeira
            (if (== (`self.PickupTypes`) 2)
              (`self.SpreadGun` (`SceneComponent.K2_GetComponentToWorld` (`self.ProjectileSpread`)))
              (`self.SpreadGun02` (`SceneComponent.K2_GetComponentToWorld` (`self.ProjectileSpread02`)))
              (`self.SpreadGun03` (`SceneComponent.K2_GetComponentToWorld` (`self.ProjectileSpread03`)))))))))
  (:`Released`
    (set `self.TaApertado?` false)))

(event `self.ReceiveAnyDamage`
  (params (Damage :type "Float (single-precision)") (DamageType :type "DamageType Object Reference") (InstigatedBy :type "Controller Object Reference") (DamageCauser :type "Actor Object Reference"))
  (bind _returnvalue (`self.K2_GetActorLocation`))
  (bind _bp_gamemode (`self.BP_GameMode`))
  ;[1 1 1] Receber o Dano
  (if (`self.Invencivel`)
    (`KismetSystemLibrary.PrintString` "You can't me touch.")
    (else
      (`PrimitiveComponent.AddImpulse` (`self.SkeletalMesh1`) (0.0 0.0 0.0) "None" false)
      (set `self.Health` (`KismetMathLibrary.FClamp` (- (`self.Health`) Damage) 0.0 (`self.MaxHealth`)))
      (set `self.Invencivel` true)
      (if (<= (`self.Health`) 0.0)
        ;[1 1 1] Qnd Toma dano  fica 3 segundos invuneravel
        (`GameplayStatics.SpawnEmitterAtLocation` "/Game/Particle/Explosion_Boss_Dead.Explosion_Boss_Dead" _returnvalue)
        (`GameplayStatics.PlaySoundAtLocation` null _returnvalue (struct) 1.0 1.0 0.0 null null null)
        (`/Game/Blueprints/GameMode_BP.PlayCamShake` _bp_gamemode null (`self.K2_GetActorLocation`))
        (`/Game/Blueprints/GameMode_BP.GameOver` _bp_gamemode)
        (`self.K2_DestroyActor`)
        (else
          (`GameplayStatics.SpawnEmitterAtLocation` "/Game/Particle/Nave_Invicible/Nave_Invicible.Nave_Invicible" (`self.K2_GetActorLocation`) (struct) (1.0 1.0 1.0) true "AutoRelease")
          (`KismetSystemLibrary.Delay` 3.0)
          (set `self.Invencivel` false))))))

(event `self.SkeletalMesh.OnComponentHit`
  (params (HitComponent :type "PrimitiveComponent Object Reference") (OtherActor :type "Actor Object Reference") (OtherComp :type "PrimitiveComponent Object Reference") (NormalImpulse :type "Vector Structure") (Hit :type "HitResult Structure (by ref)"))
  ;[1 1 1] Qnd Bate na parede volta com impulso.
  (set `self.HozSpeed` (* (* (`KismetMathLibrary.Abs` (`self.HozSpeed`)) 2.0) (.x Hit_Normal)))
  (set `self.VertSpeed` (* (* (`KismetMathLibrary.Abs` (`self.VertSpeed`)) 2.0) (.z Hit_Normal))))

(fn `BombExplosion`
  (params (SpawnTransform :type "Transform Structure"))
  (`|SpawnActorFromClass` "/Game/Bomba/Bomba.Bomba_C" SpawnTransform "AlwaysSpawn" "OverrideRootScale" null self))

(fn `MachineGun`
  (params (SpawnTransform :type "Transform Structure"))
  (locals (ProjectileColour :type "LinearColor Structure" :default (struct)))
  (`|SpawnActorFromClass` "/Game/NAVE_PROPOSTA/Tiros/Tiro_MachineGun_BP_Proposta.Tiro_MachineGun_BP_Proposta_C" SpawnTransform "Undefined" "OverrideRootScale" null (`local.ProjectileColour`) self))

(fn `Movement`
  (params (Speed :type "Float (double-precision)") (Direction :type "Float (double-precision)"))
  (returns (ReturnDirectionSpeed :type "Float (double-precision)"))
  (return (`KismetMathLibrary.FInterpTo` Speed (* (`self.MovementSpeed`) Direction) (`self.DeltaSeconds`) 6.0)))

(fn `PrimaryFire`
  (params (SpawnTransform :type "Transform Structure"))
  (locals (ProjectColour :type "LinearColor Structure" :default (struct :`G` 0.37942 :`B` 1.0)))
  (`|SpawnActorFromClass` "/Game/NAVE_PROPOSTA/Tiros/Tiro_BP_Proposta.Tiro_BP_Proposta_C" SpawnTransform "AlwaysSpawn" "OverrideRootScale" null (`local.ProjectColour`) self))

(fn `Secondary Fire`
  (params (Spawn :type "Transform Structure"))
  (`|SpawnActorFromClass` "/Game/Nave/Tiro_BP.Tiro_BP_C" Spawn "AlwaysSpawn" "OverrideRootScale" null null))

(fn `SpreadGun`
  (params (SpawnTransform :type "Transform Structure"))
  (locals (Colour :type "LinearColor Structure" :default (struct)))
  (`|SpawnActorFromClass` "/Game/NAVE_PROPOSTA/Tiros/Tiro_Spread01.Tiro_Spread01_C" SpawnTransform "AlwaysSpawn" "OverrideRootScale" null (`local.Colour`) self))

(fn `SpreadGun02`
  (params (SpawnTransform :type "Transform Structure"))
  (locals (Colour :type "LinearColor Structure" :default (struct)))
  (`|SpawnActorFromClass` "/Game/NAVE_PROPOSTA/Tiros/Tiro_Spread02.Tiro_Spread02_C" SpawnTransform "AlwaysSpawn" "OverrideRootScale" null (`local.Colour`) self))

(fn `SpreadGun03`
  (params (SpawnTransform :type "Transform Structure"))
  (locals (Colour :type "LinearColor Structure" :default (struct)))
  (`|SpawnActorFromClass` "/Game/NAVE_PROPOSTA/Tiros/Tiro_Spread03.Tiro_Spread03_C" SpawnTransform "AlwaysSpawn" "OverrideRootScale" null (`local.Colour`) self))

(fn `UserConstructionScript`
  (set `self.Health` (`self.MaxHealth`)))