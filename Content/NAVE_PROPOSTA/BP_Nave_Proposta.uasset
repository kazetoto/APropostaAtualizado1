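; Player ship pawn that rises and spins in on spawn, then moves with interpolated axis input, banking and wall-hit velocity response.
; Fire press and actor overlap share one sequence starting looping timers for primary fire, plus machine-gun or three-way spread when the overlapped actor is that pickup.
; Releasing fire clears all timers.
; Damage grants temporary invincibility; zero health triggers explosion, camera shake and GameMode game over before destroying the ship.
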(event `self.ReceiveBeginPlay`
  (bind _spawnlocation (`self.SpawnLocation`))
  ;[1 1 1] Spawn
  (bind _asgame_mode_bp (cast `/Game/Blueprints/GameMode_BP` (`GameplayStatics.GetGameMode`)))
  (set `self.BP_GameMode` _asgame_mode_bp)
  (set `self.Roll` (.yaw (`self.K2_GetActorRotation`)))
  (set `self.SpawnLocation` (`self.K2_GetActorLocation`))
  (bind (_direction _speed) (`Timeline|SpawnAnimation`)
    (:`Update`
      (`self.K2_SetActorLocation` (`KismetMathLibrary.VLerp` _spawnlocation (+ _spawnlocation (0.0 0.0 60.0)) _speed))
      (`self.K2_SetActorRotation` (`KismetMathLibrary.RLerp` (struct) (`KismetMathLibrary.MakeRotator` (+ (`self.Roll`) (`self.SpawnSpinCount`))) _speed)))
    (:`Finished`
      (set `self.MoveEnabled` true))))

(event `self.ReceiveTick`
  (params (DeltaSeconds :type "Float (single-precision)"))
  ;[1 1 1] Movement
  (set `self.DeltaSeconds` DeltaSeconds)
  (`self.K2_SetActorLocation` (+ (`self.K2_GetActorLocation`) (`KismetMathLibrary.MakeVector` (`self.VertSpeed`) (`self.HozSpeed`))) true)
  (`self.K2_SetActorRotation` (`KismetMathLibrary.RInterpTo_Constant` (`self.K2_GetActorRotation`) (`KismetMathLibrary.MakeRotator` (+ (* (`self.HozSpeed`) 7.0) (`self.Roll`))) (`self.DeltaSeconds`) 80.0)))

(event `InputAxis|Mover_Cima_Embaixo`
  (params (AxisValue :type "Float (single-precision)"))
  ;[1 1 1] Player input
  (bind _returndirectionspeed (`self.Movement` (`self.VertSpeed`) AxisValue))
  (set `self.VertSpeed` _returndirectionspeed))

(event `InputAxis|Mover`
  (params (AxisValue :type "Float (single-precision)"))
  ;[1 1 1] Player input
  (bind _returndirectionspeed (`self.Movement` (`self.HozSpeed`) AxisValue))
  (set `self.HozSpeed` _returndirectionspeed))

(event `MachGun`
  (`self.MachineGun` (`SceneComponent.K2_GetComponentToWorld` (`self.ProjectileSpawnMachineGun`)) :!label _label))

(event `self.ReceiveActorBeginOverlap`
  (params (OtherActor :type "Actor Object Reference"))
  ;[1 1 1] PrimaryFire
  (`|ExecutionSequence` :!label _label_2
    (:`then_0`
      (if (`self.MoveEnabled`)
        (set `self.PickUp Taken` 0.0)
        (`KismetSystemLibrary.K2_SetTimer` null "PrimFire" 0.2 true)
        (`self.PrimaryFire` (`SceneComponent.K2_GetComponentToWorld` (`self.ProjectileSpawn`)) :!label _label_3)))
    (:`then_1`
      (cast `/Game/PicksUps/MachineGun/PicksUP_MachineGun` OtherActor)
      (set `self.PickUp Taken` (+ (`self.PickUp Taken`) 0.0))
      (`KismetSystemLibrary.K2_SetTimer` null "MachGun" 0.2 true)
      (goto _label))
    (:`then_2`
      (cast `/Game/PicksUps/SpreadGun` OtherActor)
      (set `self.PickUP Spread` (- (`self.PickUP Spread`) -1))
      (`KismetSystemLibrary.K2_SetTimer` null "Spread01" 0.2 true)
      (`KismetSystemLibrary.K2_SetTimer` null "Spread02" 0.2 true)
      (`KismetSystemLibrary.K2_SetTimer` null "Spread03" 0.2 true)
      (`self.SpreadGun` (`SceneComponent.K2_GetComponentToWorld` (`self.ProjectileSpread`)) :!label _label_4)
      (`self.SpreadGun02` (`SceneComponent.K2_GetComponentToWorld` (`self.ProjectileSpread02`)) :!label _label_5)
      (`self.SpreadGun03` (`SceneComponent.K2_GetComponentToWorld` (`self.ProjectileSpread03`)) :!label _label_6)
      (`KismetSystemLibrary.Delay` 0.9))))

(event `Spread02`
  ;[1 1 1] PrimaryFire
  (goto _label_5))

(event `Spread01`
  ;[1 1 1] PrimaryFire
  (goto _label_4))

(event `Spread03`
  ;[1 1 1] PrimaryFire
  (goto _label_6))

(event `InputAction|PrimaryFire`
  (params (Key :type "Key Structure"))
  ;[1 1 1] PrimaryFire
  (:`Pressed`
    (goto _label_2))
  (:`Released`
    (`KismetSystemLibrary.K2_ClearTimer` null "PrimFire")
    (`KismetSystemLibrary.K2_ClearTimer` null "MachGun")
    (`KismetSystemLibrary.K2_ClearTimer` null "Spread01")
    (`KismetSystemLibrary.K2_ClearTimer` null "Spread02")
    (`KismetSystemLibrary.K2_ClearTimer` null "Spread03")))

(event `PrimFire`
  ;[1 1 1] PrimaryFire
  (goto _label_3))

(event `self.ReceiveAnyDamage`
  (params (Damage :type "Float (single-precision)") (DamageType :type "DamageType Object Reference") (InstigatedBy :type "Controller Object Reference") (DamageCauser :type "Actor Object Reference"))
  (bind _returnvalue (`self.K2_GetActorLocation`))
  (bind _bp_gamemode (`self.BP_GameMode`))
  ;[1 1 1] Receber o Dano
  (if (`self.Invencivel`)
    (`KismetSystemLibrary.PrintString` "You can't me touch.")
    (else
      (`PrimitiveComponent.AddImpulse` (`self.SkeletalMesh1`) (0.0 0.0 0.0) "None" false)
      (set `self.Health` (`KismetMathLibrary.FClamp` (- (`self.Health`) Damage) 0.0 (`self.MaxHealth`)))
      (set `self.Invencivel` true)
      (if (<= (`self.Health`) 0.0)
        (`GameplayStatics.SpawnEmitterAtLocation` "/Game/Particle/Explosion_Boss_Dead.Explosion_Boss_Dead" _returnvalue)
        (`GameplayStatics.PlaySoundAtLocation` null _returnvalue (struct) 1.0 1.0 0.0 null null null)
        (`/Game/Blueprints/GameMode_BP.PlayCamShake` _bp_gamemode null (`self.K2_GetActorLocation`))
        (`/Game/Blueprints/GameMode_BP.GameOver` _bp_gamemode)
        (`self.K2_DestroyActor`)
        (else
          (`GameplayStatics.SpawnEmitterAtLocation` "/Game/Particle/Explosion_Boss_Dead.Explosion_Boss_Dead" (`self.K2_GetActorLocation`))
          (`KismetSystemLibrary.Delay` 3.0)
          (set `self.Invencivel` false))))))

(event `self.SkeletalMesh.OnComponentHit`
  (params (HitComponent :type "PrimitiveComponent Object Reference") (OtherActor :type "Actor Object Reference") (OtherComp :type "PrimitiveComponent Object Reference") (NormalImpulse :type "Vector Structure") (Hit :type "HitResult Structure (by ref)"))
  ;[1 1 1] Qnd Bate na parede volta com impulso.
  (set `self.HozSpeed` (* (* (`KismetMathLibrary.Abs` (`self.HozSpeed`)) 0.0) (.x Hit_Normal)))
  (set `self.VertSpeed` (* (* (`KismetMathLibrary.Abs` (`self.VertSpeed`)) 2.0) (.z Hit_Normal))))

(fn `MachineGun`
  (params (SpawnTransform :type "Transform Structure"))
  (locals (ProjectileColour :type "LinearColor Structure" :default (struct)))
  (`|SpawnActorFromClass` "/Game/NAVE_PROPOSTA/Tiros/Tiro_MachineGun_BP_Proposta.Tiro_MachineGun_BP_Proposta_C" SpawnTransform "Undefined" "OverrideRootScale" null (`local.ProjectileColour`) self))

(fn `Movement`
  (params (Speed :type "Float (double-precision)") (Direction :type "Float (double-precision)"))
  (returns (ReturnDirectionSpeed :type "Float (double-precision)"))
  (return (`KismetMathLibrary.FInterpTo` Speed (* (`self.MovementSpeed`) Direction) (`self.DeltaSeconds`) 6.0)))

(fn `PrimaryFire`
  (params (SpawnTransform :type "Transform Structure"))
  (locals (ProjectColour :type "LinearColor Structure" :default (struct :`G` 0.37942 :`B` 1.0)))
  (`|SpawnActorFromClass` "/Game/NAVE_PROPOSTA/Tiros/Tiro_BP_Proposta.Tiro_BP_Proposta_C" SpawnTransform "AlwaysSpawn" "OverrideRootScale" null (`local.ProjectColour`) self))

(fn `Secondary Fire`
  (params (Spawn :type "Transform Structure"))
  (`|SpawnActorFromClass` "/Game/Nave/Tiro_BP.Tiro_BP_C" Spawn "AlwaysSpawn" "OverrideRootScale" null null))

(fn `SpreadGun`
  (params (SpawnTransform :type "Transform Structure"))
  (locals (Colour :type "LinearColor Structure" :default (struct)))
  (`|SpawnActorFromClass` "/Game/NAVE_PROPOSTA/Tiros/Tiro_Spread01.Tiro_Spread01_C" SpawnTransform "AlwaysSpawn" "OverrideRootScale" null (`local.Colour`) self))

(fn `SpreadGun02`
  (params (SpawnTransform :type "Transform Structure"))
  (locals (Colour :type "LinearColor Structure" :default (struct)))
  (`|SpawnActorFromClass` "/Game/NAVE_PROPOSTA/Tiros/Tiro_Spread02.Tiro_Spread02_C" SpawnTransform "AlwaysSpawn" "OverrideRootScale" null (`local.Colour`) self))

(fn `SpreadGun03`
  (params (SpawnTransform :type "Transform Structure"))
  (locals (Colour :type "LinearColor Structure" :default (struct)))
  (`|SpawnActorFromClass` "/Game/NAVE_PROPOSTA/Tiros/Tiro_Spread03.Tiro_Spread03_C" SpawnTransform "AlwaysSpawn" "OverrideRootScale" null (`local.Colour`) self))

(fn `UserConstructionScript`
  (set `self.Health` (`self.MaxHealth`)))